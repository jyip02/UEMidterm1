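; Actor component for a pawn that plants a random barrel actor where the player is aiming.
; TryPlant line-traces on Visibility from above the owning pawn along its control rotation out to TraceDistance, drawing a one-frame debug line.
; On a hit, Plant spawns a random class from BarrelClasses at the hit location; both outcomes print a debug message.
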(fn GetPawnOwner
  (bind _aspawn (Utilities|Casting|CastToPawn (Components|GetOwner)))
  (return _aspawn))

(fn Plant
  (params (InPlantLocation :type Vector))
  (bind _result (Utilities|Set|ToArray (Variables|Default|GetBarrelClasses)))
  (Game|SpawnActorfromClass (.OutItem (Utilities|Array|Random _result)) (Math|Transform|MakeTransform InPlantLocation "0, 0, 0" "1.000000,1.000000,1.000000") "Undefined" "MultiplyWithRoot" 0 0)
  (Development|PrintString "you planted something good "))

(fn TryPlant
  (bind _returnpawnowner (CallFunction|GetPawnOwner))
  (bind _returnvalue (Transformation|GetActorLocation _returnpawnowner))
  (bind _returnvalue_2 (Pawn|GetControlRotation _returnpawnowner :!class /Script/Engine.Pawn))
  (bind (_outhit _returnvalue_3) (Collision|LineTraceByChannel (+ _returnvalue "0.000000,0.000000,100.000000") (+ _returnvalue (* (Math|Vector|GetForwardVector (Math|Rotator|MakeRotator 0.0 (.pitch _returnvalue_2) (.yaw _returnvalue_2))) (Variables|Default|GetTraceDistance))) "TraceTypeQuery1" false 0 "ForOneFrame" true "(R=0.000000,G=0.993460,B=1.000000,A=1.000000)"))
  (if _returnvalue_3
    (CallFunction|Plant (.Location (Collision|BreakHitResult _outhit)))
    (else
      (Development|PrintString "It didn't plant"))))