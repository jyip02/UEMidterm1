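; BP_Lever is a toggle lever that reports its on or off state to the game mode.
; ActivateLever alternates through a FlipFlop, swapping the static mesh between down and up and setting the activated flag.
; Each toggle increments or decrements LeverTotal on BP_ThirdPersonGameMode, with debug prints of the state and counter.
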(event Custom|ActivateLever
  (bind _returnvalue (Game|GetGameMode))
  (bind _staticmesh (Variables|Default|GetStaticMesh))
  (Utilities|FlowControl|FlipFlop
    (:A
      (Components|StaticMesh|SetStaticMesh _staticmesh "/Game/MidtermGame/items/SM_Level_DOWN__2_.SM_Level_DOWN__2_")
      (Variables|Default|SetblsLeverActivated true)
      (Development|PrintString "Lever On")
      (bind _asbp_third_person_game_mode (Utilities|Casting|CastToBP_ThirdPersonGameMode _returnvalue))
      (bind _result (Math|Integer|IncrementInt (Variables|/Game/ThirdPerson/Blueprints/BP_ThirdPersonGameMode.BP_ThirdPersonGameMode_C|GetLeverTotal _asbp_third_person_game_mode))
        (:%20%20
          (Development|PrintString (Utilities|String|ToString(Integer) _result)))))
    (:B
      (Components|StaticMesh|SetStaticMesh _staticmesh "/Game/MidtermGame/items/SM_Lever_UP__2_.SM_Lever_UP__2_")
      (Variables|Default|SetblsLeverActivated false)
      (Development|PrintString "Lever Off")
      (bind _asbp_third_person_game_mode_2 (Utilities|Casting|CastToBP_ThirdPersonGameMode _returnvalue))
      (bind _result_2 (Math|Integer|DecrementInt (Variables|/Game/ThirdPerson/Blueprints/BP_ThirdPersonGameMode.BP_ThirdPersonGameMode_C|GetLeverTotal _asbp_third_person_game_mode_2))
        (:%20%20
          (Development|PrintString (Utilities|String|ToString(Integer) _result_2)))))))

(fn ConstructionScript)