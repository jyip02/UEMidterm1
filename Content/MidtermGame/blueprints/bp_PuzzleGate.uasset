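; Puzzle gate Blueprint that swings open once enough items have been collected.
; CollectItem increments a counter and, when it reaches the maximum, triggers OpenGate a single time through a DoOnce and prints a confirmation.
; OpenGate plays a timeline that interpolates the door's relative yaw to swing it open.
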(event Custom|Open%20Gate
  (bind _gate_rotation (Timeline|Open%20Gate%20Animation Play)
    (:Update
      (Transformation|SetRelativeRotation (Variables|Default|GetDoor) (Math|Rotator|MakeRotator 0.0 0.0 (Math|Float|Lerp 0.0 1.2e+02 _gate_rotation)) false false))))

(event Custom|Collect%20Item
  (Math|Integer|IncrementInt (Variables|Default|GetCurrentItemsCollected)
    (:%20%20
      (if (>= (Variables|Default|GetCurrentItemsCollected) (Variables|Default|GetMaxitemsCollectable))
        (Utilities|FlowControl|DoOnce false
          (:Completed
            (CallFunction|OpenGate)
            (Development|PrintString "Door is Open")))))))

(fn ConstructionScript)